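; BP_Animal is an AI-controlled animal actor whose graph handles only its death.
; OnDeath runs once, guarded by IsDead, disabling Hitbox collision and stopping the AI controller's brain logic.
; It then waits for a zero-length Delay, deferring DestroyActor to a later tick.
; Tick and the construction script are empty, and BeginPlay and overlap events are disabled placeholders.
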(event `self.ReceiveTick`
  (params (DeltaSeconds :type "Float (single-precision)")))

(event `On Death`
  (if (not (`self.Is Dead`))
    (`PrimitiveComponent.SetCollisionEnabled` (`self.Hitbox`) "NoCollision")
    (set `self.Is Dead` true)
    (`BrainComponent.StopLogic` (`AIController.BrainComponent` (`AIBlueprintHelperLibrary.GetAIController` self)) "")
    (`KismetSystemLibrary.Delay` 0.0)
    (`self.K2_DestroyActor`)))

(fn `UserConstructionScript`)